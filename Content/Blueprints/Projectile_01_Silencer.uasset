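; Silencer weapon projectile that, on activation, flies forward with speed and owner cooldown scaled by slot values, and plays a fire sound.
; A per-tick Delay loop randomizes the Noise component's rotation and sphere-traces at the projectile's position, ignoring the owner.
; The first hit ends the loop, hides the visuals and damages a struck Player, doubled for headshots.
; A BulletSpread helper exists but is uncalled here.
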(event Custom|Loop%20Logic
  (bind _returnvalue (Transformation|GetActorLocation))
  (Utilities|FlowControl|Delay 0.0 :!label _label)
  (Transformation|SetWorldRotation (Variables|Default|GetNoise) (Math|Random|RandomRotator true) false false)
  (bind (_outhit _returnvalue_2) (Collision|SphereTraceByChannel _returnvalue _returnvalue 15.0 "TraceTypeQuery1" false (Utilities|Array|MakeArray (Variables|Default|GetPlayer%20Ref)) "None"))
  (if _returnvalue_2
    (Rendering|SetVisibility (Variables|Default|GetSphere) false false)
    (bind _asplayer (Utilities|Casting|CastToPlayer (.HitActor (Collision|BreakHitResult _outhit))))
    (Default|TakeDamage _asplayer (select (== (Variables|/Game/Blueprints/Player.Player_C|GetHead _asplayer) (.HitComponent (Collision|BreakHitResult _outhit))) 20 10) (Transformation|GetActorLocation))
    (else
      (goto _label))))

(event Custom|Activate_Silencer
  (bind _slot_scales (Variables|Default|GetSlot%20Scales))
  (bind _projectilemovement (Variables|Default|GetProjectileMovement))
  (bind _output (Utilities|Array|Get(acopy) _slot_scales 1))
  (bind _returnvalue (Math|Conversions|ToFloat(Integer) _output))
  (bind _returnvalue_2 (/ _returnvalue 1e+02))
  (bind _returnvalue_3 (Math|Float|Lerp 1.5e+03 3.5e+03 _returnvalue_2))
  (Variables|/Script/Engine.MovementComponent|SetVelocity _projectilemovement (* (Transformation|GetActorForwardVector) _returnvalue_3))
  (Variables|/Script/Engine.ProjectileMovementComponent|SetMaxSpeed _projectilemovement _returnvalue_3)
  (Default|ApplyCooldown (Variables|Default|GetPlayer%20Ref) (Math|Float|Lerp 0.25 0.1 (/ (Math|Conversions|ToFloat(Integer) (Utilities|Array|Get(acopy) (Variables|Default|GetSlot%20Scales))) 1e+02)))
  (CallFunction|LoopLogic)
  (Audio|PlaySound2D "/Game/Assets/3_Sounds/Weapon_Fire.Weapon_Fire" 0.5 1.2 0.0 0 0))

(fn ConstructionScript
  (|CallParentFunction))

(fn BulletSpread
  (params (Radius :type Float%20%28single-precision%29))
  (LocalVariables|SetAngle (Math|Random|RandomFloatinRange 0.0 3.6e+02))
  (LocalVariables|SetDistance (Math|Random|RandomFloatinRange 0.0 0.0))
  (return (Math|Vector2D|MakeVector2D (* (LocalVariables|GetDistance) (Math|Trig|Cos(Degrees) (LocalVariables|GetAngle))) (* (LocalVariables|GetDistance) (Math|Trig|Sin(Degrees) (LocalVariables|GetAngle))))))