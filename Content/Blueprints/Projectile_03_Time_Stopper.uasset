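; Time Stopper projectile: a hitscan beam that freezes the shooter and any player it hits, dealing extra damage on headshots.
; A sphere trace toward the shooter's range-capped target places and stretches the Start, Middle and End meshes.
; A timeline fades the beam in and out around the freeze, while a gated tick-delay loop randomly spins the end electricity.
; Slot scales tune freeze duration and stealth, which affects beam thickness, materials and volume.
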(event Custom|Spin%20Electricity
  (Utilities|FlowControl|Delay 0.0 :!label _label)
  (Transformation|SetWorldRotation (Variables|Default|GetEnd) (Math|Random|RandomRotator true) false false)
  (Utilities|FlowControl|Gate false
    (:Exit
      (goto _label))))

(event Custom|Activate%20Time%20Stopper
  (bind _returnvalue (Transformation|GetActorLocation))
  (bind _player_ref (Variables|Default|GetPlayer%20Ref))
  (bind _slot_scales (Variables|Default|GetSlot%20Scales))
  (bind _slot_scales_2 (Variables|Default|GetSlot%20Scales))
  (bind _output (Utilities|Array|Get(acopy) _slot_scales 1))
  (bind _output_2 (Utilities|Array|Get(acopy) _slot_scales_2 1))
  (bind _bullet_target (Variables|/Game/Blueprints/Player.Player_C|GetBullet%20Target _player_ref))
  (bind _returnvalue_2 (- _bullet_target _returnvalue))
  (bind _returnvalue_3 (Math|Conversions|ToFloat(Integer) _output))
  (bind _returnvalue_4 (Math|Conversions|ToFloat(Integer) _output_2))
  (bind _returnvalue_5 (/ _returnvalue_3 1e+02))
  (bind _returnvalue_6 (/ _returnvalue_4 1e+02))
  (bind _returnvalue_7 (Math|Float|Lerp 1.0 0.2 _returnvalue_5))
  (Variables|Default|SetFreeze%20Time (Math|Float|Lerp 2.0 0.9 (/ (Math|Conversions|ToFloat(Integer) (Utilities|Array|Get(acopy) (Variables|Default|GetSlot%20Scales))) 1e+02)))
  (Default|ApplyFreeze (Variables|Default|GetPlayer%20Ref) (Variables|Default|GetFreeze%20Time))
  (Default|ApplyCooldown (Variables|Default|GetPlayer%20Ref) (Variables|Default|GetFreeze%20Time))
  (bind _returnvalue_8 (Rendering|Material|CreateDynamicMaterialInstance (Variables|Default|GetStart) 0 "/Game/Assets/1_Materials/Projectiles/Time_Stopper_Start.Time_Stopper_Start" "None" :!class /Script/Engine.PrimitiveComponent))
  (Rendering|Material|SetScalarParameterValue _returnvalue_8 "Stealth" _returnvalue_6 :!class /Script/Engine.MaterialInstanceDynamic)
  (bind _returnvalue_9 (Rendering|Material|CreateDynamicMaterialInstance (Variables|Default|GetEnd) 0 "/Game/Assets/1_Materials/Projectiles/Time_Stopper_End.Time_Stopper_End" "None" :!class /Script/Engine.PrimitiveComponent))
  (Rendering|Material|SetScalarParameterValue _returnvalue_9 "Stealth" _returnvalue_6 :!class /Script/Engine.MaterialInstanceDynamic)
  (Audio|PlaySoundatLocation "/Game/Assets/3_Sounds/Explosion.Explosion" _returnvalue "0, 0, 0" _returnvalue_7 1.0 0.0 0 0 0)
  (Audio|Components|Audio|FadeIn (Variables|Default|GetHumming) 0.2 _returnvalue_7 0.0 "Linear" :!class /Script/Engine.AudioComponent)
  (bind (_outhit _returnvalue_10) (Collision|SphereTraceByChannel _returnvalue (Math|Vector|SelectVector (+ (* (Math|Vector|Normalize _returnvalue_2) 1e+04) (Transformation|GetActorLocation)) _bullet_target (>= (Math|Vector|VectorLength _returnvalue_2) 1e+04)) 8.0 "TraceTypeQuery1" false (Utilities|Array|MakeArray _player_ref) "None" true "(R=1.000000,G=0.000000,B=0.000000,A=1.000000)" "(R=1.000000,G=0.000000,B=0.000000,A=1.000000)"))
  (if _returnvalue_10
    (Utilities|FlowControl|Sequence
      (:then_0
        (bind _asplayer (Utilities|Casting|CastToPlayer (.HitActor (Collision|BreakHitResult _outhit))))
        (Default|TakeDamage _asplayer (select (== (.HitComponent (Collision|BreakHitResult _outhit)) (Variables|/Game/Blueprints/Player.Player_C|GetHead _asplayer)) 200 70) (Transformation|GetActorLocation))
        (Default|ApplyFreeze _asplayer (- (Variables|Default|GetFreeze%20Time) 0.4))
        (Default|ApplyCooldown _asplayer (Variables|Default|GetFreeze%20Time)))
      (:then_1
        (Variables|Default|SetEnd%20Location (.Location (Collision|BreakHitResult _outhit)))
        (Variables|Default|SetMesh%20Scale (Math|Vector|VectorLength (- (.TraceStart (Collision|BreakHitResult _outhit)) (Variables|Default|GetEnd%20Location))) :!label _label)
        (Transformation|SetWorldScale3D (Variables|Default|GetMiddle) (Math|Vector|MakeVector (Variables|Default|GetMesh%20Scale) 1.0 1.0))
        (Transformation|SetWorldLocation (Variables|Default|GetEnd) (Variables|Default|GetEnd%20Location) false false)
        (CallFunction|SpinElectricity)
        (bind _returnvalue_11 (Rendering|Material|CreateDynamicMaterialInstance (Variables|Default|GetMiddle) 0 "/Game/Assets/1_Materials/Projectiles/Time_Stopper_Middle.Time_Stopper_Middle" "None" :!class /Script/Engine.PrimitiveComponent))
        (Rendering|Material|SetScalarParameterValue _returnvalue_11 "Length" (Math|Vector|VectorLength (- (Variables|Default|GetEnd%20Location) (Transformation|GetActorLocation))) :!class /Script/Engine.MaterialInstanceDynamic)
        (Rendering|Material|SetScalarParameterValue _returnvalue_11 "Stealth" (/ (Math|Conversions|ToFloat(Integer) (Utilities|Array|Get(acopy) (Variables|Default|GetSlot%20Scales) 1)) 1e+02) :!class /Script/Engine.MaterialInstanceDynamic)
        (CallFunction|BeginVisual)
        (Utilities|FlowControl|Delay (Variables|Default|GetFreeze%20Time))
        (CallFunction|EndVisual)
        (Audio|Components|Audio|FadeOut (Variables|Default|GetHumming) 0.5 0.0 "Linear" :!class /Script/Engine.AudioComponent)
        (Utilities|FlowControl|Gate false) ; enters at Close
      ))
    (else
      (Variables|Default|SetEnd%20Location (.TraceEnd (Collision|BreakHitResult _outhit)))
      (goto _label))))

(event Custom|Begin%20Visual
  (bind _middle (Variables|Default|GetMiddle))
  ;[1 1 1] Fade In/Out
  (Rendering|SetVisibility (Variables|Default|GetStart) true false)
  (bind (_direction _size) (Timeline|Fade%20In%20Animation PlayFromStart)
    (:Update
      (Transformation|SetWorldScale3D (Variables|Default|GetStart) (Math|Vector|MakeVector 1.0 (* (Math|Float|Lerp 1.0 0.4 (/ (Math|Conversions|ToFloat(Integer) (Utilities|Array|Get(acopy) (Variables|Default|GetSlot%20Scales) 1)) 1e+02)) _size) (* (Math|Float|Lerp 1.0 0.4 (/ (Math|Conversions|ToFloat(Integer) (Utilities|Array|Get(acopy) (Variables|Default|GetSlot%20Scales) 1)) 1e+02)) _size)))
      (Transformation|SetWorldScale3D _middle (Math|Vector|MakeVector (.x (Transformation|GetWorldScale _middle)) (* (Math|Float|Lerp 1.0 0.4 (/ (Math|Conversions|ToFloat(Integer) (Utilities|Array|Get(acopy) (Variables|Default|GetSlot%20Scales) 1)) 1e+02)) _size) (* (Math|Float|Lerp 1.0 0.4 (/ (Math|Conversions|ToFloat(Integer) (Utilities|Array|Get(acopy) (Variables|Default|GetSlot%20Scales) 1)) 1e+02)) _size)))
      (Transformation|SetWorldScale3D (Variables|Default|GetEnd) (Math|Vector|MakeVector (* _size 5.0) (* _size 5.0) (* _size 5.0))))
    (:Finished
      (Rendering|SetVisibility (Variables|Default|GetStart) (Utilities|Enum|Equal(Enum) _direction "Forward") false))))

(event Custom|End%20Visual
  (bind _middle (Variables|Default|GetMiddle))
  ;[1 1 1] Fade In/Out
  (bind (_direction _size) (Timeline|Fade%20In%20Animation ReverseFromEnd)
    (:Update
      (Transformation|SetWorldScale3D (Variables|Default|GetStart) (Math|Vector|MakeVector 1.0 (* (Math|Float|Lerp 1.0 0.4 (/ (Math|Conversions|ToFloat(Integer) (Utilities|Array|Get(acopy) (Variables|Default|GetSlot%20Scales) 1)) 1e+02)) _size) (* (Math|Float|Lerp 1.0 0.4 (/ (Math|Conversions|ToFloat(Integer) (Utilities|Array|Get(acopy) (Variables|Default|GetSlot%20Scales) 1)) 1e+02)) _size)))
      (Transformation|SetWorldScale3D _middle (Math|Vector|MakeVector (.x (Transformation|GetWorldScale _middle)) (* (Math|Float|Lerp 1.0 0.4 (/ (Math|Conversions|ToFloat(Integer) (Utilities|Array|Get(acopy) (Variables|Default|GetSlot%20Scales) 1)) 1e+02)) _size) (* (Math|Float|Lerp 1.0 0.4 (/ (Math|Conversions|ToFloat(Integer) (Utilities|Array|Get(acopy) (Variables|Default|GetSlot%20Scales) 1)) 1e+02)) _size)))
      (Transformation|SetWorldScale3D (Variables|Default|GetEnd) (Math|Vector|MakeVector (* _size 5.0) (* _size 5.0) (* _size 5.0))))
    (:Finished
      (Rendering|SetVisibility (Variables|Default|GetStart) (Utilities|Enum|Equal(Enum) _direction "Forward") false))))

(fn ConstructionScript
  (|CallParentFunction))