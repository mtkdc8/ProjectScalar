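; Time Stopper projectile: an instant electric beam that freezes both the firing player and any player it hits.
; A range-capped sphere trace toward the player's bullet target deals damage, with extra for headshots, and freezes the victim slightly shorter than the shooter.
; Slot scale sets freeze time.
; The beam stretches its middle mesh and material to the endpoint, randomly spins the end each tick, then hides as the hum fades.
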(event Custom|Spin%20Electricity
  (Utilities|FlowControl|Delay 0.0 :!label _label)
  (Transformation|SetWorldRotation (Variables|Default|GetEnd) (Math|Random|RandomRotator true) false false)
  (Utilities|FlowControl|Gate false
    (:Exit
      (goto _label))))

(event Custom|Activate%20Time%20Stopper
  (bind _returnvalue (Transformation|GetActorLocation))
  (bind _player_ref (Variables|Default|GetPlayer%20Ref))
  (bind _bullet_target (Variables|/Game/Blueprints/Player.Player_C|GetBullet%20Target _player_ref))
  (bind _returnvalue_2 (- _bullet_target _returnvalue))
  (Variables|Default|SetFreeze%20Time (Math|Float|Lerp 2.0 0.8 (/ (Math|Conversions|ToFloat(Integer) (Utilities|Array|Get(acopy) (Variables|Default|GetSlot%20Scales))) 1e+02)))
  (Default|FreezePlayer (Variables|Default|GetPlayer%20Ref) (Variables|Default|GetFreeze%20Time))
  (Audio|PlaySoundatLocation "/Game/Assets/3_Sounds/Explosion.Explosion" _returnvalue "0, 0, 0" 1.0 1.0 0.0 0 0 0)
  (Audio|Components|Audio|FadeIn (Variables|Default|GetHumming) 0.2 1.0 0.0 "Linear" :!class /Script/Engine.AudioComponent)
  (bind (_outhit _returnvalue_3) (Collision|SphereTraceByChannel _returnvalue (Math|Vector|SelectVector (+ (* (Math|Vector|Normalize _returnvalue_2) 1e+04) (Transformation|GetActorLocation)) _bullet_target (>= (Math|Vector|VectorLength _returnvalue_2) 1e+04)) 1e+01 "TraceTypeQuery1" false (Utilities|Array|MakeArray _player_ref) "None" true "(R=1.000000,G=0.000000,B=0.000000,A=1.000000)" "(R=1.000000,G=0.000000,B=0.000000,A=1.000000)"))
  (if _returnvalue_3
    (Utilities|FlowControl|Sequence
      (:then_0
        (bind _asplayer (Utilities|Casting|CastToPlayer (.HitActor (Collision|BreakHitResult _outhit))))
        (Default|TakeDamage _asplayer (select (== (.HitComponent (Collision|BreakHitResult _outhit)) (Variables|/Game/Blueprints/Player.Player_C|GetHead _asplayer)) 200 70))
        (Default|FreezePlayer _asplayer (- (Variables|Default|GetFreeze%20Time) 0.25)))
      (:then_1
        (Variables|Default|SetEnd%20Location (.Location (Collision|BreakHitResult _outhit)))
        (Variables|Default|SetMesh%20Scale (Math|Vector|VectorLength (- (.TraceStart (Collision|BreakHitResult _outhit)) (Variables|Default|GetEnd%20Location))) :!label _label)
        (Transformation|SetWorldScale3D (Variables|Default|GetMiddle) (Math|Vector|MakeVector (Variables|Default|GetMesh%20Scale) 1.0 1.0))
        (Transformation|SetWorldLocation (Variables|Default|GetEnd) (Variables|Default|GetEnd%20Location) false false)
        (CallFunction|SpinElectricity)
        (bind _returnvalue_4 (Rendering|Material|CreateDynamicMaterialInstance (Variables|Default|GetMiddle) 0 "/Game/Assets/1_Materials/Projectiles/Time_Stopper_Middle.Time_Stopper_Middle" "None" :!class /Script/Engine.PrimitiveComponent))
        (Rendering|Material|SetScalarParameterValue _returnvalue_4 "Length" (Math|Vector|VectorLength (- (Variables|Default|GetEnd%20Location) (Transformation|GetActorLocation))) :!class /Script/Engine.MaterialInstanceDynamic)
        (Utilities|FlowControl|Delay 2.0)
        (Rendering|SetVisibility (Variables|Default|GetStart) false false)
        (Audio|Components|Audio|FadeOut (Variables|Default|GetHumming) 0.5 0.0 "Linear" :!class /Script/Engine.AudioComponent)
        (Utilities|FlowControl|Gate false) ; enters at Close
      ))
    (else
      (Variables|Default|SetEnd%20Location (.TraceEnd (Collision|BreakHitResult _outhit)))
      (goto _label))))

(fn ConstructionScript
  (|CallParentFunction))