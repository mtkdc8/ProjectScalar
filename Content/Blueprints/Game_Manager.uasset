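; Game manager actor that sets up save data and spawns the players when play begins.
; It caches the game instance, then loads the "Scalar" save slot, first creating a default save if none exists.
; It creates additional local players based on the instance's player count, then spawns a Player at each Player_Spawn with an in-range index.
; Each pawn is possessed by the matching controller and activated with its index and a manager reference.
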(event EventBeginPlay
  ;[0.8669 0 1] Event Begin
  ;;[1 1 1] Get References for Save Data and Game Instance
  (bind _asproject_scalar_instance (Utilities|Casting|CastToProject_Scalar_Instance (Game|GetGameInstance)))
  (Variables|Default|SetScalar%20Instance%20Reference _asproject_scalar_instance)
  (bind _returnvalue (SaveGame|DoesSaveGameExist "Scalar"))
  (if _returnvalue
    _
    (else
      (bind _returnvalue_2 (SaveGame|CreateSaveGameObject "/Game/Globals/Scalar_Save_Data.Scalar_Save_Data_C"))
      (SaveGame|SaveGametoSlot _returnvalue_2 "Scalar")))
  (bind _returnvalue_3 (SaveGame|LoadGamefromSlot "Scalar"))
  (bind _asscalar_save_data (Utilities|Casting|CastToScalar_Save_Data _returnvalue_3)
    (:then
      (Variables|Default|SetSave%20Data%20Reference _asscalar_save_data)
      ;;[1 1 1] Spawn Players
      (if (!= (Variables|/Game/Globals/Project_Scalar_Instance.Project_Scalar_Instance_C|GetNum%20Players (Variables|Default|GetScalar%20Instance%20Reference)) 1)
        (for _index (range 1 (- (Math|Conversions|ToInteger(Byte) (Variables|/Game/Globals/Project_Scalar_Instance.Project_Scalar_Instance_C|GetNum%20Players (Variables|Default|GetScalar%20Instance%20Reference))) 2))
          (Class|GameplayStatics|CreatePlayer _index)))
      (bind _outactors (Actor|GetAllActorsOfClass "/Game/Blueprints/Player_Spawn.Player_Spawn_C"))
      (for _array_element _outactors
        (if (< (Variables|/Game/Blueprints/Player_Spawn.Player_Spawn_C|GetPlayer%20Index _array_element) (Math|Conversions|ToInteger(Byte) (Variables|/Game/Globals/Project_Scalar_Instance.Project_Scalar_Instance_C|GetNum%20Players (Variables|Default|GetScalar%20Instance%20Reference))))
          (bind _returnvalue_4 (Game|SpawnActorfromClass "/Game/Blueprints/Player.Player_C" (Transformation|GetActorTransform _array_element) "Undefined" 0 0))
          (Pawn|Possess (Game|GetPlayerController (Variables|/Game/Blueprints/Player_Spawn.Player_Spawn_C|GetPlayer%20Index _array_element)) _returnvalue_4)
          (Default|Activate _returnvalue_4 (Variables|/Game/Blueprints/Player_Spawn.Player_Spawn_C|GetPlayer%20Index _array_element) self))))
    (:CastFailed
      (Development|PrintString "Save Data Cast Failed!" true true "(R=1.000000,G=0.000000,B=0.000000,A=1.000000)" 8.0))))

(fn ConstructionScript)