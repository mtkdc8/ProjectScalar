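; Judgement projectile: a continuous beam weapon that damages players it hits while the owning player keeps firing.
; ActivateJudgement loops via zero-second Delay, snapping to the muzzle, sphere-tracing toward the target, stretching Middle and End, then re-aiming from the camera.
; SlotScales tune stability (random aim jitter) and range, with longer range narrowing the fade-in thickness.
; BeginVisual and EndVisual scale the beam meshes through a reversible timeline; headshots currently deal normal damage.
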(event Custom|Activate%20Judgement
  (bind _returnvalue (Transformation|GetActorLocation))
  (bind _slot_scales (Variables|Default|GetSlot%20Scales))
  (bind _player_ref (Variables|Default|GetPlayer%20Ref))
  (bind _player_ref_2 (Variables|Default|GetPlayer%20Ref))
  (bind _player_ref_3 (Variables|Default|GetPlayer%20Ref))
  (bind _returnvalue_2 (Pawn|GetControlRotation _player_ref_3 :!class /Script/Engine.Pawn))
  (bind _output (Utilities|Array|Get(acopy) _slot_scales))
  (bind _bullet_spawn_point (Variables|/Game/Blueprints/Player.Player_C|GetBullet%20Spawn%20Point _player_ref))
  (bind _bullet_spawn_point_2 (Variables|/Game/Blueprints/Player.Player_C|GetBullet%20Spawn%20Point _player_ref_2))
  (bind _returnvalue_3 (Math|Vector|GetForwardVector _returnvalue_2))
  (bind _returnvalue_4 (Transformation|GetWorldLocation _bullet_spawn_point_2))
  (bind _returnvalue_5 (Math|Conversions|ToFloat(Integer) _output))
  (bind _returnvalue_6 (Transformation|GetWorldLocation _bullet_spawn_point))
  (bind _returnvalue_7 (* _returnvalue_3 999999.0))
  (bind _returnvalue_8 (/ _returnvalue_5 1e+02))
  (bind _returnvalue_9 (Math|Float|Lerp 5.0 0.2 _returnvalue_8))
  (bind _returnvalue_10 (+ _returnvalue_7 _returnvalue_4))
  (Variables|Default|SetJudgement%20Target (Variables|/Game/Blueprints/Player.Player_C|GetBullet%20Target (Variables|Default|GetPlayer%20Ref)))
  (Transformation|SetActorTransform (Math|Transform|MakeTransform _returnvalue_6 (Math|Rotator|MakeRotator (.Roll (Math|Rotator|BreakRotator (Math|Rotator|FindLookatRotation _returnvalue_6 (Variables|Default|GetJudgement%20Target)))) (+ (.Pitch (Math|Rotator|BreakRotator (Math|Rotator|FindLookatRotation _returnvalue_6 (Variables|Default|GetJudgement%20Target)))) (* (Math|Random|RandomFloatinRange -1.0 1.0) _returnvalue_9)) (+ (.Yaw (Math|Rotator|BreakRotator (Math|Rotator|FindLookatRotation _returnvalue_6 (Variables|Default|GetJudgement%20Target)))) (* (Math|Random|RandomFloatinRange -1.0 1.0) _returnvalue_9)))) false true :!label _label)
  (bind (_outhit _returnvalue_11) (Collision|SphereTraceByChannel _returnvalue (+ (* (Math|Vector|Normalize (- (Variables|Default|GetJudgement%20Target) _returnvalue)) (Math|Float|Lerp 5e+02 2.5e+03 (/ (Math|Conversions|ToFloat(Integer) (Utilities|Array|Get(acopy) (Variables|Default|GetSlot%20Scales) 1)) 1e+02))) (Transformation|GetActorLocation)) 9.0 "TraceTypeQuery1" false (Utilities|Array|MakeArray (Variables|Default|GetPlayer%20Ref)) "None" true "(R=1.000000,G=0.000000,B=0.000000,A=1.000000)" "(R=1.000000,G=0.000000,B=0.000000,A=1.000000)"))
  (if _returnvalue_11
    (Utilities|FlowControl|Sequence
      (:then_0
        (bind _asplayer (Utilities|Casting|CastToPlayer (.HitActor (Collision|BreakHitResult _outhit))))
        (Default|TakeDamage _asplayer (select (== (.HitComponent (Collision|BreakHitResult _outhit)) (Variables|/Game/Blueprints/Player.Player_C|GetHead _asplayer)) 1 1) (Transformation|GetActorLocation)))
      (:then_1
        (Variables|Default|SetEnd%20Location (.Location (Collision|BreakHitResult _outhit)))
        (Variables|Default|SetMesh%20Scale (Math|Vector|VectorLength (- (.TraceStart (Collision|BreakHitResult _outhit)) (Variables|Default|GetEnd%20Location))) :!label _label_2)
        (Transformation|SetWorldScale3D (Variables|Default|GetMiddle) (Math|Vector|MakeVector (Variables|Default|GetMesh%20Scale) 1.0 1.0))
        (Transformation|SetRelativeLocation (Variables|Default|GetEnd) (Math|Vector|MakeVector (- (Variables|Default|GetMesh%20Scale) 1.0) 0.0 0.0) false true)
        (if (Variables|/Game/Blueprints/Player.Player_C|GetFiring%20Weapon (Variables|Default|GetPlayer%20Ref))
          (Utilities|FlowControl|Delay 0.0)
          (bind (_outhit_2 _returnvalue_12) (Collision|SphereTraceByChannel (Transformation|GetWorldLocation (Variables|/Game/Blueprints/Player.Player_C|GetPlayer%20Camera (Variables|Default|GetPlayer%20Ref))) _returnvalue_10 6.0 "TraceTypeQuery1" false (Utilities|Array|MakeArray (Variables|Default|GetPlayer%20Ref)) "None"))
          (if _returnvalue_12
            (Variables|Default|SetJudgement%20Target (.ImpactPoint (Collision|BreakHitResult _outhit_2)))
            (goto _label)
            (else
              (Variables|Default|SetJudgement%20Target _returnvalue_10)
              (goto _label)))
          (else
            (Rendering|SetVisibility (Variables|Default|GetStart) false false)))))
    (else
      (Variables|Default|SetEnd%20Location (.TraceEnd (Collision|BreakHitResult _outhit)))
      (goto _label_2))))

(event Custom|Begin%20Visual
  (bind _middle (Variables|Default|GetMiddle))
  ;[1 1 1] Fade In/Out
  (Rendering|SetVisibility (Variables|Default|GetStart) true false)
  (bind (_direction _size) (Timeline|Fade%20In%20Animation PlayFromStart)
    (:Update
      (Transformation|SetWorldScale3D (Variables|Default|GetStart) (Math|Vector|MakeVector 1.0 (* (Math|Float|Lerp 1.0 0.4 (/ (Math|Conversions|ToFloat(Integer) (Utilities|Array|Get(acopy) (Variables|Default|GetSlot%20Scales) 1)) 1e+02)) _size) (* (Math|Float|Lerp 1.0 0.4 (/ (Math|Conversions|ToFloat(Integer) (Utilities|Array|Get(acopy) (Variables|Default|GetSlot%20Scales) 1)) 1e+02)) _size)))
      (Transformation|SetWorldScale3D _middle (Math|Vector|MakeVector (.x (Transformation|GetWorldScale _middle)) (* (Math|Float|Lerp 1.0 0.4 (/ (Math|Conversions|ToFloat(Integer) (Utilities|Array|Get(acopy) (Variables|Default|GetSlot%20Scales) 1)) 1e+02)) _size) (* (Math|Float|Lerp 1.0 0.4 (/ (Math|Conversions|ToFloat(Integer) (Utilities|Array|Get(acopy) (Variables|Default|GetSlot%20Scales) 1)) 1e+02)) _size)))
      (Transformation|SetWorldScale3D (Variables|Default|GetEnd) (Math|Vector|MakeVector (* _size 5.0) (* _size 5.0) (* _size 5.0))))
    (:Finished
      (Rendering|SetVisibility (Variables|Default|GetStart) (Utilities|Enum|Equal(Enum) _direction "Forward") false))))

(event Custom|End%20Visual
  (bind _middle (Variables|Default|GetMiddle))
  ;[1 1 1] Fade In/Out
  (bind (_direction _size) (Timeline|Fade%20In%20Animation ReverseFromEnd)
    (:Update
      (Transformation|SetWorldScale3D (Variables|Default|GetStart) (Math|Vector|MakeVector 1.0 (* (Math|Float|Lerp 1.0 0.4 (/ (Math|Conversions|ToFloat(Integer) (Utilities|Array|Get(acopy) (Variables|Default|GetSlot%20Scales) 1)) 1e+02)) _size) (* (Math|Float|Lerp 1.0 0.4 (/ (Math|Conversions|ToFloat(Integer) (Utilities|Array|Get(acopy) (Variables|Default|GetSlot%20Scales) 1)) 1e+02)) _size)))
      (Transformation|SetWorldScale3D _middle (Math|Vector|MakeVector (.x (Transformation|GetWorldScale _middle)) (* (Math|Float|Lerp 1.0 0.4 (/ (Math|Conversions|ToFloat(Integer) (Utilities|Array|Get(acopy) (Variables|Default|GetSlot%20Scales) 1)) 1e+02)) _size) (* (Math|Float|Lerp 1.0 0.4 (/ (Math|Conversions|ToFloat(Integer) (Utilities|Array|Get(acopy) (Variables|Default|GetSlot%20Scales) 1)) 1e+02)) _size)))
      (Transformation|SetWorldScale3D (Variables|Default|GetEnd) (Math|Vector|MakeVector (* _size 5.0) (* _size 5.0) (* _size 5.0))))
    (:Finished
      (Rendering|SetVisibility (Variables|Default|GetStart) (Utilities|Enum|Equal(Enum) _direction "Forward") false))))

(fn ConstructionScript
  (|CallParentFunction))