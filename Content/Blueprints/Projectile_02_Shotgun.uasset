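; Shotgun projectile Blueprint that fires an instant burst of hitscan pellets from the player's aim and applies a cooldown.
; Two slot scales set pellet count and spread, with each pellet sphere-traced toward a random point within a circle around the aim point.
; Player hits deal damage, doubled for the Head component.
; Each pellet adds a stretched static mesh as a tracer, hidden after a short delay.
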(event Custom|Activate_Shotgun
  (bind _returnvalue (Transformation|GetActorLocation))
  (bind _player_ref (Variables|Default|GetPlayer%20Ref))
  (bind _returnvalue_2 (Pawn|GetControlRotation _player_ref :!class /Script/Engine.Pawn))
  (Variables|Default|SetSpread (Math|Float|Lerp 2e+03 5e+02 (/ (Math|Conversions|ToFloat(Integer) (Utilities|Array|Get(acopy) (Variables|Default|GetSlot%20Scales) 1)) 1e+02)))
  (Default|ApplyCooldown (Variables|Default|GetPlayer%20Ref) 0.5)
  (for _index (range 1 (Math|Float|Round (Math|Float|Lerp 4.0 12.0 (/ (Math|Conversions|ToFloat(Integer) (Utilities|Array|Get(acopy) (Variables|Default|GetSlot%20Scales))) 1e+02))))
    (bind _point (CallFunction|BulletSpread))
    (bind (_outhit _returnvalue_3) (Collision|SphereTraceByChannel (Transformation|GetActorLocation) (+ (+ (* (Math|Vector|GetForwardVector _returnvalue_2) (Variables|Default|GetBulletDistance)) (Transformation|GetWorldLocation (Variables|/Game/Blueprints/Player.Player_C|GetPlayer%20Camera _player_ref))) (* (Math|Vector|GetRightVector _returnvalue_2) (.X (Math|Vector2D|BreakVector2D _point))) (* (Math|Vector|GetUpVector _returnvalue_2) (.Y (Math|Vector2D|BreakVector2D _point)))) 3.0 "TraceTypeQuery1" false 0 "None"))
    (if _returnvalue_3
      (Variables|Default|SetEnd%20Location (.Location (Collision|BreakHitResult _outhit)))
      (Utilities|FlowControl|Sequence
        (:then_0
          (bind _asplayer (Utilities|Casting|CastToPlayer (.HitActor (Collision|BreakHitResult _outhit))))
          (Default|TakeDamage _asplayer (select (== (.HitComponent (Collision|BreakHitResult _outhit)) (Variables|/Game/Blueprints/Player.Player_C|GetHead _asplayer)) 16 8) (Transformation|GetActorLocation)))
        (:then_1
          (bind _returnvalue_4 (AddComponent|AddStaticMeshComponent false (Math|Transform|MakeTransform "0, 0, 0") :!label _label))
          (Utilities|Array|Add (Variables|Default|GetShrapnel%20Meshes) _returnvalue_4)
          (Transformation|SetWorldTransform _returnvalue_4 (Math|Transform|MakeTransform _returnvalue (Math|Rotator|FindLookatRotation _returnvalue (.TraceEnd (Collision|BreakHitResult _outhit))) (Math|Vector|MakeVector (Math|Vector|VectorLength (- (.TraceStart (Collision|BreakHitResult _outhit)) (Variables|Default|GetEnd%20Location))) 0.3 0.3)) false false)))
      (else
        (Variables|Default|SetEnd%20Location (.TraceEnd (Collision|BreakHitResult _outhit)))
        (goto _label))))
  (Utilities|FlowControl|Delay 0.5)
  (Rendering|SetVisibility (Variables|Default|GetShrapnel%20Meshes) false false))

(fn ConstructionScript
  (|CallParentFunction))

(fn BulletSpread
  (LocalVariables|SetAngle (Math|Random|RandomFloatinRange 0.0 3.6e+02))
  (LocalVariables|SetDistance (Math|Random|RandomFloatinRange 0.0 (Variables|Default|GetSpread)))
  (return (Math|Vector2D|MakeVector2D (* (LocalVariables|GetDistance) (Math|Trig|Cos(Degrees) (LocalVariables|GetAngle))) (* (LocalVariables|GetDistance) (Math|Trig|Sin(Degrees) (LocalVariables|GetAngle))))))